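; Player controller that handles pawn movement input and sets up a custom crosshair mouse cursor.
; On BeginPlay it caches the controlled pawn, shows the cursor locked to the window in Game and UI mode, and assigns WBP_Cursor as the Crosshairs cursor widget.
; The Enhanced Input IA_Move action feeds MoveInput, which moves the cached pawn along right and forward vectors derived from control rotation.
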(event `EnhancedInput|/Game/Core/Game/IA_Move`
  (params (ActionValue :type "Vector2D Structure") (ElapsedSeconds :type "Float (double-precision)") (TriggeredSeconds :type "Float (double-precision)") (InputAction :type "InputAction Object Reference" :default "/Game/Core/Game/IA_Move.IA_Move"))
  (:`Triggered`
    (`self.MoveInput` ActionValue_X ActionValue_Y)))

(event `self.ReceiveBeginPlay`
  (`self.SetupVariables`)
  ; Set game to have cursor visible and lock it inside window
  (set `self.bShowMouseCursor` true)
  (`WidgetBlueprintLibrary.SetInputMode_GameAndUIEx` self null "LockAlways" false)
  (`self.ChangeToCustomCursor`))

(fn `ChangeToCustomCursor`
  (bind _returnvalue (`|CreateWidget` "/Game/Core/UI/WBP_Cursor.WBP_Cursor_C"))
  (`self.SetMouseCursorWidget` "Crosshairs" _returnvalue)
  (set `self.CurrentMouseCursor` "Crosshairs"))

(fn `MoveInput`
  (params (X :type "Float (double-precision)") (Y :type "Float (double-precision)"))
  (bind (_returnvalue_roll _returnvalue_pitch _returnvalue_yaw) (`KismetMathLibrary.BreakRotator` (`self.GetControlRotation`)))
  (bind (_returnvalue_roll_2 _returnvalue_pitch_2 _returnvalue_yaw_2) (`KismetMathLibrary.BreakRotator` (`self.GetControlRotation`)))
  ; Move Right Left
  (set `self.Move_X` X)
  (set `self.Move_Y` Y)
  (`Pawn.AddMovementInput` (`self.Controlled Pawn`) (`KismetMathLibrary.GetRightVector` (`KismetMathLibrary.MakeRotator` _returnvalue_roll_2 0.0 _returnvalue_yaw_2)) (`self.Move_X`) false)
  ; Move Forward Backward
  (`Pawn.AddMovementInput` (`self.Controlled Pawn`) (`KismetMathLibrary.GetForwardVector` (`KismetMathLibrary.MakeRotator` 0.0 0.0 _returnvalue_yaw)) (`self.Move_Y`) false))

(fn `SetupVariables`
  (set `self.Controlled Pawn` (`self.K2_GetPawn`)))

(fn `UserConstructionScript`)