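; BP_BWSEnemySpawner is a spawner actor that periodically spawns BP_BWSBaseBot enemies around the player.
; BeginPlay caches the player character and starts a looping timer at SpawnFrequency.
; Each tick of the timer runs the EQS_BWSFindEnemySpawnLocation query from the player, setting its ring radius from SpawnRingRadius.
; When the query finishes, a bot spawns at a random returned point, adjusting for collisions but always spawning.
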(event `OnQueryFinished`
  (params (QueryInstance :type "EnvQueryInstanceBlueprintWrapper Object Reference") (QueryStatus :type "EEnvQueryStatus Enum" :default "Processing"))
  ; Find Player -> Set looped timer -> Get point around player iwth EQS - > Set EQS Doughnut radius -> Bind to EQS Finish event to spawn actor at random Point from query
  (bind _resultlocations (`EnvQueryInstanceBlueprintWrapper.GetQueryResultsAsLocations` QueryInstance))
  (`|SpawnActorFromClass` "/Game/Core/Characters/BP_BWSBaseBot.BP_BWSBaseBot_C" (`KismetMathLibrary.MakeTransform` (`KismetArrayLibrary.Array_Random` _resultlocations)) "AdjustIfPossibleButAlwaysSpawn" "MultiplyWithRoot" null null))

(event `Spawn`
  ; Find Player -> Set looped timer -> Get point around player iwth EQS - > Set EQS Doughnut radius -> Bind to EQS Finish event to spawn actor at random Point from query
  (bind _returnvalue (`EnvQueryManager.RunEQSQuery` "/Game/Core/Gameplay/Spawner/EQS/EQS_BWSFindEnemySpawnLocation.EQS_BWSFindEnemySpawnLocation" (`self.Cached Player Actor`) "RandomBest25Pct"))
  (`EnvQueryInstanceBlueprintWrapper.SetNamedParam` _returnvalue (`self.Ring Radius Name`) (`self.Spawn Ring Radius`))
  (add `EnvQueryInstanceBlueprintWrapper.OnQueryFinishedEvent` _returnvalue (delegate `OnQueryFinished`)))

(event `self.ReceiveBeginPlay`
  ; Find Player -> Set looped timer -> Get point around player iwth EQS - > Set EQS Doughnut radius -> Bind to EQS Finish event to spawn actor at random Point from query
  (bind _returnvalue (`GameplayStatics.GetActorOfClass` "/Game/Core/Characters/BP_BWSPlayerCharacter.BP_BWSPlayerCharacter_C"))
  (set `self.Cached Player Actor` _returnvalue)
  (`KismetSystemLibrary.K2_SetTimerDelegate` (delegate `Spawn`) (`self.Spawn Frequency`) true))

(event `self.ReceiveActorBeginOverlap`
  (params (OtherActor :type "Actor Object Reference")))

(fn `UserConstructionScript`
  (`parent.UserConstructionScript`))