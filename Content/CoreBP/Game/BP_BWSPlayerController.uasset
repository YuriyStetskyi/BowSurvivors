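; Player controller for a mouse-aimed shooter: it moves the controlled pawn, turns it toward the cursor and fires arrows.
; Each tick it line-traces the deprojected mouse position into the world and snaps the pawn's yaw toward the hit.
; Move input is relative to control yaw; shooting spawns BP_BWSProjectile ahead of the pawn with a forward impulse.
; On BeginPlay it caches the pawn, locks the visible mouse to the window and applies a crosshair widget cursor.
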(event `EnhancedInput|/Game/CoreBP/Game/Inputs/IA_Shoot`
  (params (ActionValue :type Boolean) (ElapsedSeconds :type "Float (double-precision)") (TriggeredSeconds :type "Float (double-precision)") (InputAction :type "InputAction Object Reference" :default "/Game/CoreBP/Game/Inputs/IA_Shoot.IA_Shoot"))
  (:`Triggered`
    (`KismetSystemLibrary.PrintString` (`KismetStringLibrary.Conv_VectorToString` (`self.Cursor Location In World`)) true true (struct :`G` 1.0 :`A` 1.0) 1.0)
    (`self.ShootArrowAtDirection` (`self.GetActorForwardVector` (`self.Controlled Pawn`)) 1500.0)))

(event `EnhancedInput|/Game/CoreBP/Game/Inputs/IA_Move`
  (params (ActionValue :type "Vector2D Structure") (ElapsedSeconds :type "Float (double-precision)") (TriggeredSeconds :type "Float (double-precision)") (InputAction :type "InputAction Object Reference" :default "/Game/CoreBP/Game/Inputs/IA_Move.IA_Move"))
  (:`Triggered`
    (`self.MoveInput` ActionValue_X ActionValue_Y)))

(event `self.ReceiveBeginPlay`
  (`self.SetupVariables`)
  ; Set game to have cursor visible and lock it inside window
  (set `self.bShowMouseCursor` true)
  (`WidgetBlueprintLibrary.SetInputMode_GameAndUIEx` self null "LockAlways" false)
  (`self.ChangeToCustomCursor`))

(event `self.ReceiveTick`
  (params (DeltaSeconds :type "Float (single-precision)"))
  ; Get Character and Mouse (in world) location every frame
  (bind _newparam (`self.FindMouseLocationProjectedOntoWorld`))
  (set `self.Cursor Location In World` _newparam)
  (set `self.Curret Character Location` (`self.K2_GetActorLocation` (`self.Controlled Pawn`)))
  (`self.RotateCharacterToMouseCursor` (`self.Curret Character Location`) (`self.Cursor Location In World`)))

(fn `ChangeToCustomCursor`
  (bind _returnvalue (`|CreateWidget` "/Game/CoreBP/UI/WBP_Cursor.WBP_Cursor_C"))
  (`self.SetMouseCursorWidget` "Crosshairs" _returnvalue)
  (set `self.CurrentMouseCursor` "Crosshairs"))

(fn `FindMouseLocationProjectedOntoWorld`
  (returns (NewParam :type "Vector Structure"))
  (bind (_locationx _locationy) (`self.GetMousePosition`))
  (bind (_worldposition _worlddirection) (`GameplayStatics.DeprojectScreenToWorld` self (`KismetMathLibrary.MakeVector2D` _locationx _locationy)))
  (bind (_outhits _returnvalue) (`KismetSystemLibrary.LineTraceMulti` _worldposition (* _worlddirection 100000) "TraceTypeQuery1"))
  (if _returnvalue
    (return (`.Location` (`GameplayStatics.BreakHitResult` (`|GetArrayItem` _outhits))))))

(fn `MoveInput`
  (params (X :type "Float (double-precision)") (Y :type "Float (double-precision)"))
  (bind (_returnvalue_roll _returnvalue_pitch _returnvalue_yaw) (`KismetMathLibrary.BreakRotator` (`self.GetControlRotation`)))
  (bind (_returnvalue_roll_2 _returnvalue_pitch_2 _returnvalue_yaw_2) (`KismetMathLibrary.BreakRotator` (`self.GetControlRotation`)))
  ; Move Right Left
  (set `self.Move_X` X)
  (set `self.Move_Y` Y)
  (`Pawn.AddMovementInput` (`self.Controlled Pawn`) (`KismetMathLibrary.GetRightVector` (`KismetMathLibrary.MakeRotator` _returnvalue_roll_2 0.0 _returnvalue_yaw_2)) (`self.Move_X`) false)
  ; Move Forward Backward
  (`Pawn.AddMovementInput` (`self.Controlled Pawn`) (`KismetMathLibrary.GetForwardVector` (`KismetMathLibrary.MakeRotator` 0.0 0.0 _returnvalue_yaw)) (`self.Move_Y`) false))

(fn `RotateCharacterToMouseCursor`
  (params (CharacterLocation :type "Vector Structure") (MouseLocation :type "Vector Structure"))
  (locals (`Cleaned Character Location` :type "Vector Structure") (`Cleaned Mouse Location` :type "Vector Structure"))
  (set `local.Cleaned Character Location` (`KismetMathLibrary.MakeVector` CharacterLocation_X CharacterLocation_Y))
  (set `local.Cleaned Mouse Location` (`KismetMathLibrary.MakeVector` MouseLocation_X MouseLocation_Y))
  (`self.K2_SetActorRotation` (`self.Controlled Pawn`) (`KismetMathLibrary.FindLookAtRotation` (`local.Cleaned Character Location`) (`local.Cleaned Mouse Location`)) false))

(fn `SetupVariables`
  (set `self.Controlled Pawn` (`self.K2_GetPawn`)))

(fn `ShootArrowAtDirection`
  (params (`Direction (starts from pawn)` :type "Vector Structure") (`Impulse Strength` :type "Float (double-precision)"))
  (bind (_returnvalue_location _returnvalue_rotation _returnvalue_scale) (`KismetMathLibrary.BreakTransform` (`self.GetTransform` (`self.Controlled Pawn`))))
  (bind _returnvalue (`|SpawnActorFromClass` "/Game/CoreBP/Gameplay/Combat/BP_BWSProjectile.BP_BWSProjectile_C" (`KismetMathLibrary.MakeTransform` (+ (* (`self.GetActorForwardVector` (`self.Controlled Pawn`)) 100.0) _returnvalue_location) _returnvalue_rotation _returnvalue_scale) "Undefined" "MultiplyWithRoot" self 1.0 null))
  (`PrimitiveComponent.AddImpulse` (`/Game/CoreBP/Gameplay/Combat/BP_BWSProjectile.ProjectileMesh` _returnvalue) (* (`local.Impulse Strength`) (`local.Direction (starts from pawn)`)) "None" true)
  (return))

(fn `UserConstructionScript`)