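; BP_BWSPlayerController is a player controller that carries debug hotkeys for testing the player character.
; Raw K, G and F key events cast player character 0 to BP_BWSPlayerCharacter and call its test functions to display weapon stats, add gold and apply damage.
; The attack input action only prints a placeholder string, and the show-stats action is left empty.
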(event `EnhancedInput|/Game/Game/Controllers/Inputs/IA_ShowStats`
  (params (ActionValue :type Boolean) (ElapsedSeconds :type "Float (double-precision)") (TriggeredSeconds :type "Float (double-precision)") (InputAction :type "InputAction Object Reference" :default "/Game/Game/Controllers/Inputs/IA_ShowStats.IA_ShowStats")))

(event `Key|K`
  (params (Key :type "Key Structure"))
  (:`Pressed`
    (bind _asbp_bwsplayer_character (cast `/Game/Game/Characters/BP_BWSPlayerCharacter` (`GameplayStatics.GetPlayerCharacter` 0)))
    (`BWSPlayerCharacter.Test_DisplayWeaponStats` _asbp_bwsplayer_character)))

(event `Key|G`
  (params (Key :type "Key Structure"))
  (:`Pressed`
    (bind _asbp_bwsplayer_character (cast `/Game/Game/Characters/BP_BWSPlayerCharacter` (`GameplayStatics.GetPlayerCharacter` 0)))
    (`BWSPlayerCharacter.Test_AddGold` _asbp_bwsplayer_character 25.0)))

(event `Key|F`
  (params (Key :type "Key Structure"))
  (:`Pressed`
    (bind _asbp_bwsplayer_character (cast `/Game/Game/Characters/BP_BWSPlayerCharacter` (`GameplayStatics.GetPlayerCharacter` 0)))
    (`BWSPlayerCharacter.Test_TakeDamage` _asbp_bwsplayer_character 20.0)))

(event `EnhancedInput|/Game/Game/Controllers/Inputs/IA_Attack`
  (params (ActionValue :type "Float (double-precision)") (ElapsedSeconds :type "Float (double-precision)") (TriggeredSeconds :type "Float (double-precision)") (InputAction :type "InputAction Object Reference" :default "/Game/Game/Controllers/Inputs/IA_Attack.IA_Attack"))
  (:`Triggered`
    (`KismetSystemLibrary.PrintString` "Hello")))

(fn `UserConstructionScript`)